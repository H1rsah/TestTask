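; Player character Blueprint that handles movement, camera look, aiming, running and attack input.
; Movement follows control rotation, with strafing allowed only in the aim state, which also sets walk speed and blocks starting a run.
; Run input switches max walk speed between run and walk values.
; A BoxingComponent, initialized with the character on BeginPlay, receives the Fire press to start attacks.
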(event `self.ReceiveBeginPlay`
  (`/Game/Blueprints/BoxingComponent.Initialize` (`self.BoxingComponent`) self))

(event `InputAxis|Mouse Turn`
  (params (AxisValue :type "Float (single-precision)"))
  ;[1 1 1] Movement/Turning
  (`self.AddControllerYawInput` AxisValue))

(event `InputAxis|Move F/B`
  (params (AxisValue :type "Float (single-precision)"))
  (bind (_returnvalue_roll _returnvalue_pitch _returnvalue_yaw) (`KismetMathLibrary.BreakRotator` (`self.GetControlRotation`)))
  ;[1 1 1] Movement/Turning
  (`self.AddMovementInput` (`KismetMathLibrary.GetForwardVector` (`KismetMathLibrary.MakeRotator` 0.0 0.0 _returnvalue_yaw)) AxisValue))

(event `InputAxis|Mouse Up`
  (params (AxisValue :type "Float (single-precision)"))
  ;[1 1 1] Movement/Turning
  (`self.AddControllerPitchInput` AxisValue))

(event `InputAxis|Move R/L`
  (params (AxisValue :type "Float (single-precision)"))
  (bind (_returnvalue_roll _returnvalue_pitch _returnvalue_yaw) (`KismetMathLibrary.BreakRotator` (`self.GetControlRotation`)))
  ;[1 1 1] Movement/Turning
  (if (`|EnumEquality` (`self.State`) "NewEnumerator1")
    (`self.AddMovementInput` (`KismetMathLibrary.GetRightVector` (`KismetMathLibrary.MakeRotator` _returnvalue_roll 0.0 _returnvalue_yaw)) AxisValue)))

(event `InputAction|Aim`
  (params (Key :type "Key Structure"))
  (:`Pressed`
    (set `self.State` "NewEnumerator1")
    (set `CharacterMovementComponent.MaxWalkSpeed` (`self.SpeedWalk`) (`self.CharacterMovement`)))
  (:`Released`
    (set `self.State` "NewEnumerator0")))

(event `InputAction|Run/Walk`
  (params (Key :type "Key Structure"))
  (bind _charactermovement (`self.CharacterMovement`))
  (:`Pressed`
    (if (`|EnumInequality` (`self.State`) "NewEnumerator1")
      (set `self.IsRunning` true)
      (set `CharacterMovementComponent.MaxWalkSpeed` (`self.SpeedRun`) _charactermovement)))
  (:`Released`
    (set `self.IsRunning` false)
    (set `CharacterMovementComponent.MaxWalkSpeed` (`self.SpeedWalk`) _charactermovement)))

(event `InputAction|Fire`
  (params (Key :type "Key Structure"))
  (:`Pressed`
    (`/Game/Blueprints/BoxingComponent.StartAttack` (`self.BoxingComponent`))))

(fn `UserConstructionScript`)