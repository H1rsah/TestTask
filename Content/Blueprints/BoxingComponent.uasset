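; Boxing component that plays random attack montages on its owning character.
; Initialization requires more than one listed attack, and StartAttack fires only when the character is in a specific state and not already hitting.
; When identical attacks are disallowed, selection rerolls until it differs from the last index, which a timer later resets.
; Montage completion releases the hitting lock, while StopAttack stops the current attack's montage and clears it.
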(event `Initialize`
  (params (Character :type "/Game/Blueprints/BP_Character Object Reference"))
  (set `self.CharacterRef` Character)
  (if (> (`KismetArrayLibrary.Array_Length` (`self.AttackList`)) 1)
    (set `self.IsInitialized` true)))

(event `StopAttack`
  (bind (_currentattack_type _currentattack_animmontage) (break `/Game/Structures/S_BoxingAttacks` (`self.CurrentAttack`)))
  (`Character.StopAnimMontage` (`self.CharacterRef`) _currentattack_animmontage)
  (`self.ClearAttack`))

(event `StartAttack`
  (if (and (`self.IsInitialized`) (`KismetSystemLibrary.IsValid` (`self.CharacterRef`)))
    (if (and (not (`self.IsHitting`)) (`|EnumEquality` (`/Game/Blueprints/BP_Character.State` (`self.CharacterRef`)) "NewEnumerator1"))
      (bind _attacktype (`self.SelectRandomAttackFromList`))
      (`self.Hit` (`.AnimMontage_5_116042A940E0DFF1C6A3E7B42E2A054E` (break `/Game/Structures/S_BoxingAttacks` _attacktype))))))

(event `Hit`
  (params (MontageToPlay :type "AnimMontage Object Reference"))
  (`|PlayMontage` (`Character.Mesh` (`self.CharacterRef`)) MontageToPlay
    (:`then`
      (set `self.IsHitting` true)
      (if (not (`self.IsIdenticalAttacksAreAllowed`))
        (bind _returnvalue (`KismetSystemLibrary.K2_SetTimerDelegate` (delegate `ResetTimer`) (`self.IdenticalAttackTimer`)))
        (set `self.IdenticalAttackTimerHandle` _returnvalue)))
    (:`OnCompleted`
      (set `self.IsHitting` false)
      (if (`self.IsIdenticalAttacksAreAllowed`)
        (`self.ClearAttack`)))))

(event `ResetTimer`
  (`self.ClearAttack`)
  (set `self.IdenticalAttackTimerHandle` (struct))
  (set `self.LastAttackIndex` -1))

(fn `ClearAttack`
  (set `self.CurrentAttack` (make `/Game/Structures/S_BoxingAttacks` "NewEnumerator2" null)))

(fn `GetRandomIndex`
  (returns (Index :type Integer))
  (return (`KismetMathLibrary.RandomInteger` (`KismetArrayLibrary.Array_Length` (`self.AttackList`)))))

(fn `SelectRandomAttackFromList`
  (returns (AttackType :type "/Game/Structures/S_BoxingAttacks Structure"))
  (locals (LocalIndex :type Integer :default 0))
  (if (`self.IsIdenticalAttacksAreAllowed`)
    (return (`|GetArrayItem` (`self.AttackList`) (`self.GetRandomIndex`)))
    (else
      (bind _output_get (set `local.LocalIndex` (`self.GetRandomIndex`)))
      (while (== _output_get (`self.LastAttackIndex`))
        (set `local.LocalIndex` (`self.GetRandomIndex`)))
      (set `self.LastAttackIndex` (`local.LocalIndex`))
      (return (`|GetArrayItem` (`self.AttackList`) (`local.LocalIndex`))))))